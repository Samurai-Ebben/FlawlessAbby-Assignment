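; BP_PickItem is a world pickup actor that hands its ItemData to the third-person character's inventory.
; Its Trigger component tracks the overlapping BP_ThirdPersonCharacter, clearing the reference when a character of that class leaves.
; The PickUp event only proceeds when the interactor is that tracked character, then calls AddItem on its inventory component.
; The actor destroys itself only if the item is successfully added.
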(event OnComponentBeginOverlap(Trigger)
  (params (OverlappedComponent :type Primitive%20Component%20Object%20Reference) (OtherActor :type Actor%20Object%20Reference) (OtherComp :type Primitive%20Component%20Object%20Reference) (OtherBodyIndex :type Integer) (bFromSweep :type Boolean) (SweepResult :type Hit%20Result%20Structure%20%28by%20ref%29))
  (bind _asbp_third_person_character (Utilities|Casting|CastToBP_ThirdPersonCharacter OtherActor))
  (Utilities|IsValid _asbp_third_person_character
    (:Is%20Valid
      (Variables|Default|SetOverlappingPawn _asbp_third_person_character))))

(event OnComponentEndOverlap(Trigger)
  (params (OverlappedComponent :type Primitive%20Component%20Object%20Reference) (OtherActor :type Actor%20Object%20Reference) (OtherComp :type Primitive%20Component%20Object%20Reference) (OtherBodyIndex :type Integer))
  (bind _asbp_third_person_character (Utilities|Casting|CastToBP_ThirdPersonCharacter OtherActor))
  (Utilities|IsValid _asbp_third_person_character
    (:Is%20Valid
      (Variables|Default|SetOverlappingPawn 0))))

(event EventBeginPlay)

(event Collision|EventActorBeginOverlap
  (params (OtherActor :type Actor%20Object%20Reference)))

(event EventPickUp
  (params (Interactor :type Actor%20Object%20Reference))
  (if (== Interactor (Variables|Default|GetOverlappingPawn))
    (bind _asbp_third_person_character (Utilities|Casting|CastToBP_ThirdPersonCharacter Interactor))
    (bind _added (Default|AddItem (Variables|/Game/ThirdPerson/Blueprints/BP_ThirdPersonCharacter.BP_ThirdPersonCharacter_C|GetBPC_InventoryComp _asbp_third_person_character) (Variables|Default|GetItemData)))
    (if _added
      (Actor|DestroyActor))))

(fn ConstructionScript)
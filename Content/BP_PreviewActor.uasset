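; BP_PreviewActor renders an isolated view of its own static mesh through a scene capture, with functions to rotate and zoom that view.
; On BeginPlay, SceneCaptureComponent2D is restricted to show only this actor's components, excluding child actors.
; AdjustZoom changes the capture's FOV within a clamped range.
; RotateRelative adds roll and pitch to the mesh from X and Y deltas.
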(event EventBeginPlay
  (Rendering|SceneCapture|ShowOnlyActorComponents (Variables|Default|GetSceneCaptureComponent2D) self false))

(event Collision|EventActorBeginOverlap
  (params (OtherActor :type Actor%20Object%20Reference)))

(event EventTick
  (params (DeltaSeconds :type Float%20%28single-precision%29)))

(fn ConstructionScript)

(fn AdjustZoom
  (params (Delta :type Float%20%28double-precision%29))
  (bind _scenecapturecomponent2d (Variables|Default|GetSceneCaptureComponent2D))
  (Variables|/Script/Engine.SceneCaptureComponent2D|SetFOVAngle _scenecapturecomponent2d (Math|Float|Clamp(Float) (+ Delta (Variables|/Script/Engine.SceneCaptureComponent2D|GetFOVAngle _scenecapturecomponent2d)) 1e+01 1.2e+02)))

(fn RotateRelative
  (params (DeltaX :type Float%20%28double-precision%29) (DeltaY :type Float%20%28double-precision%29))
  (Transformation|AddRelativeRotation (Variables|Default|GetStaticMesh) (Math|Rotator|MakeRotator DeltaX DeltaY 0.0) false false))
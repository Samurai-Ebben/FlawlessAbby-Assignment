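; Inventory component that stores items in the InvItems array and exposes AddItem for adding new ones.
; AddItem scans the first four slots, writes the item into the first invalid one, fires the OnInvUpdated dispatcher and returns true.
; When all four slots hold valid items it returns false without broadcasting.
; The event graph has no active logic.
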(event EventBeginPlay)

(event EventTick
  (params (DeltaSeconds :type Float%20%28single-precision%29)))

(fn AddItem
  (params (NewItem :type DA%20Item%20Object%20Reference))
  (for _index (range 0 3)
    (if (not (Utilities|IsValid (Utilities|Array|Get(acopy) (Variables|Default|GetInvItems) _index)))
      (Utilities|Array|SetArrayElem (Variables|Default|GetInvItems) _index NewItem)
      (Default|CallOnInvUpdated)
      (return true)))
  (return false))
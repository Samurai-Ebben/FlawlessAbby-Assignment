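; BP_NPC is a non-player character that shows dialogue to the player one line at a time when interacted with.
; Each Interact event advances an index into its dialogue array, creating a WB_Dialouge widget with itself as speaker if none exists and setting the widget's text.
; Once the index passes the last line, it removes the widget, clears the reference and resets the index so the conversation can replay.
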(event EventBeginPlay)

(event Collision|EventActorBeginOverlap
  (params (OtherActor :type Actor%20Object%20Reference)))

(event EventTick
  (params (DeltaSeconds :type Float%20%28single-precision%29)))

(event EventInteract
  (params (PlayerLoc :type Vector :default "0, 0, 0"))
  (Math|Integer|IncrementInt (Variables|Default|GetDiaIndex)
    (:%20%20
      (if (< (Variables|Default|GetDiaIndex) (Utilities|Array|Length (Variables|Default|GetDialouge)))
        (Variables|Default|GetDiaWidget
          (:then
            _)
          (:else
            (bind _returnvalue (UserInterface|CreateWidget "/Game/Widgets/WB_Dialouge.WB_Dialouge_C" (Game|GetPlayerController 0) self))
            (bind _output_get (Variables|Default|SetDiaWidget _returnvalue))
            (UserInterface|Viewport|AddtoViewport _output_get 0)))
        (Rendering|Components|TextRender|SetText (Variables|/Game/Widgets/WB_Dialouge.WB_Dialouge_C|GetTxtDia (Variables|Default|GetDiaWidget)) (Utilities|Text|ToText(String) (Utilities|Array|Get(acopy) (Variables|Default|GetDialouge) (Variables|Default|GetDiaIndex))))
        (else
          (Widget|RemovefromParent (Variables|Default|GetDiaWidget))
          (Variables|Default|SetDiaIndex -1)
          (Variables|Default|SetDiaWidget 0))))))

(fn ConstructionScript)